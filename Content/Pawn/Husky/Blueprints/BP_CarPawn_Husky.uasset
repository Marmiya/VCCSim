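; BP_CarPawn_Husky is a drivable Chaos wheeled vehicle pawn for the Husky, carrying a Lidar sensor initialized in the construction script.
; On possession by a player controller it adds the Husky Enhanced Input mapping context.
; Steering is remapped from 0–1 to -1–1, and pedal values are inverted and clamped.
; The Brake action drives throttle, Throttle drives brake, and Clutch feeds the handbrake.
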(event Custom|movee
  (Class|CarPawn|Move))

(event Input|EnhancedActionEvents|EnhancedInputActionIA_Husky_Brake
  (params (ActionValue :type Float%20%28double-precision%29) (ElapsedSeconds :type Float%20%28double-precision%29) (TriggeredSeconds :type Float%20%28double-precision%29) (InputAction :type Input%20Action%20Object%20Reference :default "/VCCSim/Pawn/Husky/Input/IA_Husky_Brake.IA_Husky_Brake"))
  (bind _normalized_pedal (CallFunction|ProcessPedalInput ActionValue))
  (Class|ChaosVehicleMovementComponent|SetThrottleInput (Variables|Default|GetChaosWheeledVehicleMovement) _normalized_pedal))

(event Input|EnhancedActionEvents|EnhancedInputActionIA_Husky_Clutch
  (params (ActionValue :type Boolean) (ElapsedSeconds :type Float%20%28double-precision%29) (TriggeredSeconds :type Float%20%28double-precision%29) (InputAction :type Input%20Action%20Object%20Reference :default "/VCCSim/Pawn/Husky/Input/IA_Husky_Clutch.IA_Husky_Clutch"))
  (Class|ChaosVehicleMovementComponent|SetHandbrakeInput (Variables|Default|GetChaosWheeledVehicleMovement) ActionValue))

(event Input|EnhancedActionEvents|EnhancedInputActionIA_Husky_Steering
  (params (ActionValue :type Float%20%28double-precision%29) (ElapsedSeconds :type Float%20%28double-precision%29) (TriggeredSeconds :type Float%20%28double-precision%29) (InputAction :type Input%20Action%20Object%20Reference :default "/VCCSim/Pawn/Husky/Input/IA_Husky_Steering.IA_Husky_Steering"))
  (bind _normalized_steering (CallFunction|ProcessSteeringInput ActionValue))
  (Class|ChaosVehicleMovementComponent|SetSteeringInput (Variables|Default|GetChaosWheeledVehicleMovement) _normalized_steering))

(event Input|EnhancedActionEvents|EnhancedInputActionIA_Husky_Throttle
  (params (ActionValue :type Float%20%28double-precision%29) (ElapsedSeconds :type Float%20%28double-precision%29) (TriggeredSeconds :type Float%20%28double-precision%29) (InputAction :type Input%20Action%20Object%20Reference :default "/VCCSim/Pawn/Husky/Input/IA_Husky_Throttle.IA_Husky_Throttle"))
  (bind _normalized_pedal (CallFunction|ProcessPedalInput ActionValue))
  (Class|ChaosVehicleMovementComponent|SetBrakeInput (Variables|Default|GetChaosWheeledVehicleMovement) _normalized_pedal))

(event EventBeginPlay)

(event Collision|EventActorBeginOverlap
  (params (OtherActor :type Actor%20Object%20Reference)))

(event EventTick
  (params (DeltaSeconds :type Float%20%28single-precision%29)))

(event EventPossessed
  (params (NewController :type Controller%20Object%20Reference))
  (bind _asplayer_controller (Utilities|Casting|CastToPlayerController NewController))
  (Input|AddMappingContext (PlayerController|LocalPlayerSubsystems|GetEnhancedInputLocalPlayerSubsystem _asplayer_controller) "/VCCSim/Pawn/Husky/Input/IM_Husky_InputMapping.IM_Husky_InputMapping" 1 "(bIgnoreAllPressedKeysUntilRelease=True,bForceImmediately=False,bNotifyUserSettings=False)"))

(fn ConstructionScript
  (bind _lidar (Variables|Default|GetLidar))
  (Class|LidarComponent|InitSensor _lidar)
  (Variables|/Script/VCCSim.LidarComponent|SetMeshHolder _lidar (Variables|Default|GetInsMeshHolder)))

(fn ProcessSteeringInput
  (params (Raw%20Steering%20Value :type Float%20%28double-precision%29))
  (return (Math|Float|Clamp(Float) (* (- Raw%20Steering%20Value 0.5) 2.0) -1.0)))

(fn ProcessPedalInput
  (params (Raw%20Steering%20Value :type Float%20%28double-precision%29))
  (return (Math|Float|Clamp(Float) (Math|Float|Absolute(Float) (- Raw%20Steering%20Value 1.0)))))